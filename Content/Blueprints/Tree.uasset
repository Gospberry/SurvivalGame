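; Tree actor that randomizes its look on spawn and can fall down.
; BeginPlay randomizes yaw and scale, then runs a debug-drawn visibility trace whose end multiplies, rather than offsets, location by the scaled up vector.
; On a hit, it moves the mesh there and creates dynamic materials with a random green color, though the parameter name is None.
; FallDown enables mesh physics, then destroys the actor after a short delay.
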(event Custom|FallDown
  (Physics|SetSimulatePhysics (Variables|Default|GetStaticMesh) true)
  (Utilities|FlowControl|Delay 4.0)
  (Actor|DestroyActor))

(event EventBeginPlay
  (bind _scene (Variables|Default|GetScene))
  (bind _returnvalue (Transformation|GetWorldLocation _scene))
  (Transformation|SetActorRotation (Math|Rotator|MakeRotator 0.0 0.0 (Math|Random|RandomFloatinRange -1.9e+02 1.9e+02)))
  (Transformation|SetActorScale3D (Math|Vector|MakeVector (Math|Random|RandomFloatinRange 2.0 2.5) (Math|Random|RandomFloatinRange 2.0 2.5) (Math|Random|RandomFloatinRange 2.0 2.5)))
  (bind (_outhit _returnvalue_2) (Collision|LineTraceByChannel _returnvalue (* _returnvalue (* (Math|Vector|GetUpVector _scene) 5e+04)) "TraceTypeQuery1" false 0 "ForDuration" true "(R=1.000000,G=0.000000,B=0.000000,A=1.000000)" "(R=0.000000,G=1.000000,B=0.000000,A=1.000000)" 1e+01))
  (if _returnvalue_2
    (Transformation|SetWorldLocation (Variables|Default|GetStaticMesh) (.Location (Collision|BreakHitResult _outhit)) false false)
    (for _index (range 0 2)
      (bind _returnvalue_3 (Rendering|Material|CreateDynamicMaterialInstance (Variables|Default|GetStaticMesh) _index "/Engine/MapTemplates/Materials/BasicAsset01.BasicAsset01" "None" :!class /Script/Engine.PrimitiveComponent))
      (Rendering|Material|SetVectorParameterValue _returnvalue_3 "None" (Utilities|Struct|MakeLinearColor (Math|Random|RandomFloatinRange 0.3 0.5) 0.8 0.0 1.0) :!class /Script/Engine.MaterialInstanceDynamic))))

(fn ConstructionScript)